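; BP_Spiketrap is a spike trap actor that applies a radial impulse to its own Box component when any actor overlaps it.
; It caches the BP_Player instance at BeginPlay and centers the short-range, constant-falloff impulse on that player's location.
; The overlapping actor is never checked, as the player cast is disconnected, along with an unused radial force node.
; It contains no damage logic.
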(event EventBeginPlay
  (Utilities|FlowControl|Sequence
    (:then_0
      (bind _returnvalue (Actor|GetActorOfClass "/Game/Blueprints/BP_Player.BP_Player_C"))
      (Variables|Default|SetBP_playerref _returnvalue))))

(event Collision|EventActorBeginOverlap
  (params (OtherActor :type Actor%20Object%20Reference))
  (Physics|AddRadialImpulse (Variables|Default|GetBox) (Transformation|GetActorLocation (Variables|Default|GetBP_playerref)) 4e+01 1e+03 "RIF_Constant" false))

(event EventTick
  (params (DeltaSeconds :type Float%20%28single-precision%29)))

(fn ConstructionScript)