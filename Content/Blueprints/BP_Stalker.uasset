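; BP_Stalker is an actor that trails BP_Player by heading toward where the player was some frames earlier.
; Tick keeps a rolling buffer of player locations capped at FrameDelay, and MoveToPlayer takes the oldest as the goal.
; A looping timer, set to the current frame delta, teleports it Speed units toward the goal without sweeping.
; Within AcceptableRadius, it clears the timer and picks the next goal.
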(event Custom|MoveToPlayer
  (Variables|Default|SetGoal (Utilities|Array|Get(acopy) (Variables|Default|GetPlayerLoc)))
  (bind _returnvalue (Utilities|Time|SetTimerbyEvent (delegate Custom|Move) (Utilities|Time|GetWorldDeltaSeconds) true))
  (Variables|Default|SetMoveTimer _returnvalue))

(event Custom|Move
  (Transformation|AddActorWorldOffset (* (Variables|Default|GetSpeed) (Math|Vector|GetUnitDirection(Vector) (Transformation|GetActorLocation) (Variables|Default|GetGoal))) false true)
  (if (<= (Math|Vector|Distance(Vector) (Transformation|GetActorLocation) (Variables|Default|GetGoal)) (Variables|Default|GetAcceptableRadius))
    (Utilities|Time|ClearandInvalidateTimerbyHandle (Variables|Default|GetMoveTimer))
    (CallFunction|MovetoPlayer)))

(event EventBeginPlay
  (Pawn|SpawnDefaultController)
  (bind _returnvalue (Actor|GetActorOfClass "/Game/Blueprints/BP_Player.BP_Player_C"))
  (Variables|Default|SetPlayerRef _returnvalue)
  (Utilities|FlowControl|Delay 1.0)
  (CallFunction|MovetoPlayer))

(event EventTick
  (params (DeltaSeconds :type Float%20%28single-precision%29))
  (Utilities|Array|Add (Variables|Default|GetPlayerLoc) (Transformation|GetActorLocation (Variables|Default|GetPlayerRef)))
  (if (> (Utilities|Array|Length (Variables|Default|GetPlayerLoc)) (Variables|Default|GetFrameDelay))
    (Utilities|Array|RemoveIndex (Variables|Default|GetPlayerLoc))))

(fn ConstructionScript)